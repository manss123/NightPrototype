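; Villager NPC that implements interaction functions to offer a single Talk option with a fixed greeting, asking to face the interactor.
; Focus events highlight InteractClickBox through custom depth stencil and a material swap, restoring the material cached at BeginPlay.
; The approach point is computed on a horizontal radius around the villager, on the side facing the first player's pawn.
; The Interact event itself is empty.
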(event `self.Interact`
  (params (Interactor :type "Actor Object Reference")))

(event `self.OnInteractFocusBegin`
  (params (Interactor :type "Actor Object Reference"))
  (bind _interactclickbox (`self.InteractClickBox`))
  (`PrimitiveComponent.SetRenderCustomDepth` _interactclickbox true)
  (`PrimitiveComponent.SetCustomDepthStencilValue` _interactclickbox 252)
  (`PrimitiveComponent.SetMaterial` _interactclickbox 0 (`self.HighlightMaterial `)))

(event `self.ReceiveBeginPlay`
  (set `self.OriginalMaterial ` (`PrimitiveComponent.GetMaterial` (`self.InteractClickBox`) 0)))

(event `self.OnInteractFocusEnd`
  (params (Interactor :type "Actor Object Reference"))
  (bind _interactclickbox (`self.InteractClickBox`))
  (`PrimitiveComponent.SetRenderCustomDepth` _interactclickbox false)
  (`PrimitiveComponent.SetMaterial` _interactclickbox 0 (`self.OriginalMaterial `)))

(fn `CanInteract`
  (params (Interactor :type "Actor Object Reference"))
  (returns (ReturnValue :type Boolean))
  (return true))

(fn `GetDialogueText`
  (returns (ReturnValue :type Text))
  (return "Hello Stranger!"))

(fn `GetInteractDistance`
  (returns (ReturnValue :type "Float (single-precision)"))
  (return 80.0))

(fn `GetInteractionOptions`
  (returns (ReturnValue :type "Array of DWInteractionOption Structure"))
  (return (`|MakeArray` (make `DWInteractionOption` "Talk" "Talk"))))

(fn `GetInteractLocation`
  (returns (ReturnValue :type "Vector Structure"))
  (bind _returnvalue (`self.K2_GetActorLocation`))
  (return (+ (* (`KismetMathLibrary.Normal` (`KismetMathLibrary.MakeVector` (.x (- (`self.K2_GetActorLocation` (`GameplayStatics.GetPlayerPawn` 0)) _returnvalue)) (.y (- (`self.K2_GetActorLocation` (`GameplayStatics.GetPlayerPawn` 0)) _returnvalue)))) (`self.InteractionApproachRadius`)) _returnvalue)))

(fn `GetInteractText`
  (returns (ReturnValue :type Text))
  (return "Talk to Villager"))

(fn `ShouldFaceInteractor`
  (returns (ReturnValue :type Boolean))
  (return true))

(fn `ShouldShowDialogue`
  (returns (ReturnValue :type Boolean))
  (return true))

(fn `UserConstructionScript`)