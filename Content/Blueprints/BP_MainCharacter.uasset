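; BP_MainCharacter is the main character Blueprint, and its graph handles stepped camera rotation around the character.
; Pressing Q or E turns the SpringArm left or right by a fixed yaw increment in world space.
; Each press keeps the current pitch, zeroes roll and snaps instantly, with no interpolation.
; The construction script is empty, and the graph contains no movement logic.
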(event `Key|Q`
  (params (Key :type "Key Structure"))
  (bind _springarm (`self.SpringArm`))
  (:`Pressed`
    (`SceneComponent.K2_SetWorldRotation` _springarm (`KismetMathLibrary.MakeRotator` 0.0 (.pitch (`SceneComponent.K2_GetComponentRotation` _springarm)) (- (.yaw (`SceneComponent.K2_GetComponentRotation` _springarm)) 15.0)) false false)))

(event `Key|E`
  (params (Key :type "Key Structure"))
  (bind _springarm (`self.SpringArm`))
  (:`Pressed`
    (`SceneComponent.K2_SetWorldRotation` _springarm (`KismetMathLibrary.MakeRotator` 0.0 (.pitch (`SceneComponent.K2_GetComponentRotation` _springarm)) (+ (.yaw (`SceneComponent.K2_GetComponentRotation` _springarm)) 15.0)) false false)))

(fn `UserConstructionScript`)